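; BP_PawnCamera is an early-stage camera Blueprint with keyboard-driven test logic for its PlayerCamera and CameraBump components.
; Pressing W prints PlayerCamera's world location offset by 100 on every axis, and releasing it moves the camera by that offset.
; Pressing D only prints CameraBump's world transform.
; BeginPlay, overlap, Tick and the construction script are empty.
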(event `Key|D`
  (params (Key :type "Key Structure"))
  (:`Pressed`
    (`KismetSystemLibrary.PrintString` (`KismetStringLibrary.Conv_TransformToString` (`SceneComponent.K2_GetComponentToWorld` (`self.CameraBump`))))))

(event `Key|W`
  (params (Key :type "Key Structure"))
  (bind _returnvalue_location (`KismetMathLibrary.BreakTransform` (`SceneComponent.K2_GetComponentToWorld` (`self.PlayerCamera`))))
  (bind _returnvalue (+ _returnvalue_location 100.0))
  (:`Pressed`
    (`KismetSystemLibrary.PrintString` (`KismetStringLibrary.Conv_VectorToString` _returnvalue)))
  (:`Released`
    (`SceneComponent.K2_SetWorldTransform` (`self.PlayerCamera`) (`KismetMathLibrary.MakeTransform` _returnvalue) false false)))

(fn `UserConstructionScript`)