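; BP_ItemMain is a pickup item actor that the player collects by pressing E while nearby.
; Its Sphere overlap events enable input for player controller 0 when a ThirdPersonCharacter enters and disable it on exit, gating the E key.
; On E, it casts the overlapping actor to ThirdPersonCharacter, passes ItemInfo to that character's PickUpItemEvent, then destroys itself.
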(event `Key|E`
  (params (Key :type "Key Structure"))
  (:`Pressed`
    (bind _asthird_person_character (cast `/Game/ThirdPersonBP/Blueprints/ThirdPersonCharacter` (stale `self.Sphere.OnComponentBeginOverlap` OtherActor)))
    (`/Game/ThirdPersonBP/Blueprints/ThirdPersonCharacter.PickUp Item Event` _asthird_person_character (`self.ItemInfo`))
    (`self.K2_DestroyActor`)))

(event `self.Sphere.OnComponentBeginOverlap`
  (params (OverlappedComponent :type "PrimitiveComponent Object Reference") (OtherActor :type "Actor Object Reference") (OtherComp :type "PrimitiveComponent Object Reference") (OtherBodyIndex :type Integer) (bFromSweep :type Boolean) (SweepResult :type "HitResult Structure (by ref)"))
  ;[1 1 1] Check if the one who overlapping is our character
  (cast `/Game/ThirdPersonBP/Blueprints/ThirdPersonCharacter` OtherActor)
  ;[1 1 1] Enable input access if it is a player
  (`self.EnableInput` (`GameplayStatics.GetPlayerController` 0)))

(event `self.Sphere.OnComponentEndOverlap`
  (params (OverlappedComponent :type "PrimitiveComponent Object Reference") (OtherActor :type "Actor Object Reference") (OtherComp :type "PrimitiveComponent Object Reference") (OtherBodyIndex :type Integer))
  ;[1 1 1] Our player is not overlapping
  (cast `/Game/ThirdPersonBP/Blueprints/ThirdPersonCharacter` OtherActor)
  ;[1 1 1] Disable input
  (`self.DisableInput` (`GameplayStatics.GetPlayerController` 0)))

(fn `UserConstructionScript`)